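; BP_GrabActor is an actor built around a BPCGrabComponent, with Grab, Release and UpdateApproach events for grabbing.
; UpdateApproach calls StartApproachBoth on the component and branches on its result, with nothing attached to the branch.
; Grab and Release are empty.
; Disconnected nodes sketch a looping frame-delta timer for UpdateApproach, its clearing, and a StopApproachBoth call, but none of them run.
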(event Custom|UpdateApproach
  (bind _isapproached (Default|StartApproachBoth (Variables|Default|GetBPC_GrabComponent)))
  (if _isapproached
    _))

(event EventGrab
  (params (Motion%20Controller :type Motion%20Controller%20Component%20Object%20Reference)))

(event EventRelease)

(fn ConstructionScript)