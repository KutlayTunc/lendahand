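; VR grabbable actuator whose physics-driven handle follows a motion controller around a single axis while held.
; Grab disables handle physics and starts a looping per-frame timer; Release clears it and restores physics.
; The timer waits on BPCGrabComponent's hand approach, selects the hand animation, then runs SwitchOnAxis.
; SwitchOnAxis applies local Roll or Pitch from an interpolated look-at dot product; the Yaw logic is unconnected.
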(event Custom|UpdateApproach
  (bind _isapproached (Default|StartApproachHandOnly (Variables|Default|GetBPC_GrabComponent)))
  (if _isapproached
    (Default|SelectAnimAfterApproachHand (Variables|Default|GetBPC_GrabComponent))
    (Utilities|SwitchonAxis)))

(event EventGrab
  (params (Motion%20Controller :type Motion%20Controller%20Component%20Object%20Reference))
  (Variables|Default|SetMotion%20Controller Motion%20Controller)
  (Physics|SetSimulatePhysics (Variables|Default|GetActuatorHandle) false)
  (bind _returnvalue (Utilities|Time|SetTimerbyEvent (delegate Custom|UpdateApproach) (Utilities|Time|GetWorldDeltaSeconds) true))
  (Variables|Default|SetGrabTimer _returnvalue))

(event EventRelease
  (Utilities|Time|ClearandInvalidateTimerbyHandle (Variables|Default|GetGrabTimer))
  (Physics|SetSimulatePhysics (Variables|Default|GetActuatorHandle) true))

(fn ConstructionScript)