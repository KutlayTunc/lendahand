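; VR-style hand Blueprint that tracks per-segment finger flex, overlap and blocked states for grab curls.
; Ten finger colliders flag segments touching actors with a BPC_GrabComponent, with each 03 collider also flagging its 02 segment.
; StartGrabCurls sets HandAnim and starts a looping timer that feeds an interpolated grip value into HandleCurls.
; HandleCurls raises lower flex values past a small threshold, clearing blocked flags without halting those segments.
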(event `self.ReceiveBeginPlay`
  (`self.SetFingerCapsules`))

(event `SetFingerCapsules`
  (set `self.FingersCollisions` (`|MakeMap` "NewEnumerator0" (`self.ColThumb02`) "NewEnumerator2" (`self.ColIndex02`) "NewEnumerator4" (`self.ColMiddle02`) "NewEnumerator6" (`self.ColRing02`) "NewEnumerator8" (`self.ColPinky02`) "NewEnumerator1" (`self.ColThumb03`) "NewEnumerator3" (`self.ColIndex03`) "NewEnumerator5" (`self.ColMiddle03`) "NewEnumerator7" (`self.ColRing03`) "NewEnumerator9" (`self.ColPinky03`) :!type "/Game/Core/Hand/E_TriggerIndexes Enum"))
  (bind _enumvalue (foreach `/Game/Core/Hand/E_TriggerIndexes` false)
    (:`LoopBody`
      (`BlueprintMapLibrary.Map_Add` (`self.FingersBlocked`) _enumvalue)
      (`BlueprintMapLibrary.Map_Add` (`self.FingersFlex`) _enumvalue)
      (`BlueprintMapLibrary.Map_Add` (`self.FingersOverlapping`) _enumvalue))))

(event `StartGrabCurls`
  (set `self.HandAnim` "NewEnumerator1")
  (bind _returnvalue (`KismetSystemLibrary.K2_SetTimerDelegate` (delegate `UpdateGrabCurl`) (`GameplayStatics.GetWorldDeltaSeconds`) true))
  (set `self.GrabCurlTimer` _returnvalue))

(event `UpdateGrabCurl`
  (bind _returnvalue (`KismetMathLibrary.FInterpTo_Constant` 0.0 1.0 (`GameplayStatics.GetWorldDeltaSeconds`) 5.0))
  (`self.HandleCurls` _returnvalue)
  (if (>= _returnvalue 1.0)
    (`KismetSystemLibrary.K2_ClearAndInvalidateTimerHandle` (`self.GrabCurlTimer`))))

(event `self.ColThumb02.OnComponentBeginOverlap`
  (params (OverlappedComponent :type "PrimitiveComponent Object Reference") (OtherActor :type "Actor Object Reference") (OtherComp :type "PrimitiveComponent Object Reference") (OtherBodyIndex :type Integer) (bFromSweep :type Boolean) (SweepResult :type "HitResult Structure (by ref)"))
  (`self.SetFingerOverlapping` true "NewEnumerator0" OtherActor))

(event `self.ColIndex02.OnComponentBeginOverlap`
  (params (OverlappedComponent :type "PrimitiveComponent Object Reference") (OtherActor :type "Actor Object Reference") (OtherComp :type "PrimitiveComponent Object Reference") (OtherBodyIndex :type Integer) (bFromSweep :type Boolean) (SweepResult :type "HitResult Structure (by ref)"))
  (`self.SetFingerOverlapping` true "NewEnumerator2" OtherActor))

(event `self.ColMiddle02.OnComponentBeginOverlap`
  (params (OverlappedComponent :type "PrimitiveComponent Object Reference") (OtherActor :type "Actor Object Reference") (OtherComp :type "PrimitiveComponent Object Reference") (OtherBodyIndex :type Integer) (bFromSweep :type Boolean) (SweepResult :type "HitResult Structure (by ref)"))
  (`self.SetFingerOverlapping` true "NewEnumerator4" OtherActor))

(event `self.ColRing02.OnComponentBeginOverlap`
  (params (OverlappedComponent :type "PrimitiveComponent Object Reference") (OtherActor :type "Actor Object Reference") (OtherComp :type "PrimitiveComponent Object Reference") (OtherBodyIndex :type Integer) (bFromSweep :type Boolean) (SweepResult :type "HitResult Structure (by ref)"))
  (`self.SetFingerOverlapping` true "NewEnumerator6" OtherActor))

(event `self.ColPinky02.OnComponentBeginOverlap`
  (params (OverlappedComponent :type "PrimitiveComponent Object Reference") (OtherActor :type "Actor Object Reference") (OtherComp :type "PrimitiveComponent Object Reference") (OtherBodyIndex :type Integer) (bFromSweep :type Boolean) (SweepResult :type "HitResult Structure (by ref)"))
  (`self.SetFingerOverlapping` true "NewEnumerator8" OtherActor))

(event `self.ColThumb03.OnComponentBeginOverlap`
  (params (OverlappedComponent :type "PrimitiveComponent Object Reference") (OtherActor :type "Actor Object Reference") (OtherComp :type "PrimitiveComponent Object Reference") (OtherBodyIndex :type Integer) (bFromSweep :type Boolean) (SweepResult :type "HitResult Structure (by ref)"))
  (`self.SetFingerOverlapping` true "NewEnumerator0" OtherActor)
  (`self.SetFingerOverlapping` true "NewEnumerator1" OtherActor))

(event `self.ColIndex03.OnComponentBeginOverlap`
  (params (OverlappedComponent :type "PrimitiveComponent Object Reference") (OtherActor :type "Actor Object Reference") (OtherComp :type "PrimitiveComponent Object Reference") (OtherBodyIndex :type Integer) (bFromSweep :type Boolean) (SweepResult :type "HitResult Structure (by ref)"))
  (`self.SetFingerOverlapping` true "NewEnumerator2" OtherActor)
  (`self.SetFingerOverlapping` true "NewEnumerator3" OtherActor))

(event `self.ColMiddle03.OnComponentBeginOverlap`
  (params (OverlappedComponent :type "PrimitiveComponent Object Reference") (OtherActor :type "Actor Object Reference") (OtherComp :type "PrimitiveComponent Object Reference") (OtherBodyIndex :type Integer) (bFromSweep :type Boolean) (SweepResult :type "HitResult Structure (by ref)"))
  (`self.SetFingerOverlapping` true "NewEnumerator4" OtherActor)
  (`self.SetFingerOverlapping` true "NewEnumerator5" OtherActor))

(event `self.ColRing03.OnComponentBeginOverlap`
  (params (OverlappedComponent :type "PrimitiveComponent Object Reference") (OtherActor :type "Actor Object Reference") (OtherComp :type "PrimitiveComponent Object Reference") (OtherBodyIndex :type Integer) (bFromSweep :type Boolean) (SweepResult :type "HitResult Structure (by ref)"))
  (`self.SetFingerOverlapping` true "NewEnumerator6" OtherActor)
  (`self.SetFingerOverlapping` true "NewEnumerator7" OtherActor))

(event `self.ColPinky03.OnComponentBeginOverlap`
  (params (OverlappedComponent :type "PrimitiveComponent Object Reference") (OtherActor :type "Actor Object Reference") (OtherComp :type "PrimitiveComponent Object Reference") (OtherBodyIndex :type Integer) (bFromSweep :type Boolean) (SweepResult :type "HitResult Structure (by ref)"))
  (`self.SetFingerOverlapping` true "NewEnumerator8" OtherActor)
  (`self.SetFingerOverlapping` true "NewEnumerator9" OtherActor))

(fn `ClearCurls`
  (locals (ArrElement :type "/Game/Core/Hand/E_TriggerIndexes Enum"))
  (bind _keys (`BlueprintMapLibrary.Map_Keys` (`self.FingersBlocked`)))
  (for _array_element _keys
    (set `local.ArrElement` _array_element)
    (`BlueprintMapLibrary.Map_Add` (`self.FingersBlocked`) (`local.ArrElement`))
    (`BlueprintMapLibrary.Map_Add` (`self.FingersOverlapping`) (`local.ArrElement`))
    (`BlueprintMapLibrary.Map_Add` (`self.FingersFlex`) (`local.ArrElement`))))

(fn `FingerMovement`
  (params (FingerIndex :type "/Game/Core/Hand/E_TriggerIndexes Enum" :default "NewEnumerator0") (AlphaInput :type "Float (double-precision)"))
  (if (> (`KismetMathLibrary.Abs` (- (`local.AlphaInput`) (`BlueprintMapLibrary.Map_Find` (`self.FingersFlex`) (`local.FingerIndex`)))) 0.05)
    (`BlueprintMapLibrary.Map_Add` (`self.FingersFlex`) (`local.FingerIndex`) (`local.AlphaInput`))))

(fn `HandleCurls`
  (params (GripCurl :type "Float (double-precision)"))
  (locals (ArrElement :type "/Game/Core/Hand/E_TriggerIndexes Enum"))
  (bind _keys (`BlueprintMapLibrary.Map_Keys` (`self.FingersBlocked`)))
  (for _array_element _keys
    (set `local.ArrElement` _array_element)
    (if (> (`local.GripCurl`) (`BlueprintMapLibrary.Map_Find` (`self.FingersFlex`) (`local.ArrElement`)))
      (if (`BlueprintMapLibrary.Map_Find` (`self.FingersBlocked`) (`local.ArrElement`))
        (`BlueprintMapLibrary.Map_Add` (`self.FingersBlocked`) (`local.ArrElement`))
        (`self.FingerMovement` (`local.ArrElement`) (`local.GripCurl`))
        (else
          (`self.FingerMovement` (`local.ArrElement`) (`local.GripCurl`)))))))

(fn `SetFingerFlexes`
  (params (Thumb :type "Float (double-precision)") (Index :type "Float (double-precision)") (Middle :type "Float (double-precision)") (Ring :type "Float (double-precision)") (Pinky :type "Float (double-precision)"))
  (`BlueprintMapLibrary.Map_Add` (`self.FingersFlex`) "NewEnumerator0" (`local.Thumb`))
  (`BlueprintMapLibrary.Map_Add` (`self.FingersFlex`) "NewEnumerator1" (`local.Thumb`))
  (`BlueprintMapLibrary.Map_Add` (`self.FingersFlex`) "NewEnumerator2" (`local.Index`))
  (`BlueprintMapLibrary.Map_Add` (`self.FingersFlex`) "NewEnumerator3" (`local.Index`))
  (`BlueprintMapLibrary.Map_Add` (`self.FingersFlex`) "NewEnumerator4" (`local.Middle`))
  (`BlueprintMapLibrary.Map_Add` (`self.FingersFlex`) "NewEnumerator5" (`local.Middle`))
  (`BlueprintMapLibrary.Map_Add` (`self.FingersFlex`) "NewEnumerator6" (`local.Ring`))
  (`BlueprintMapLibrary.Map_Add` (`self.FingersFlex`) "NewEnumerator7" (`local.Ring`))
  (`BlueprintMapLibrary.Map_Add` (`self.FingersFlex`) "NewEnumerator8" (`local.Pinky`))
  (`BlueprintMapLibrary.Map_Add` (`self.FingersFlex`) "NewEnumerator9" (`local.Pinky`)))

(fn `SetFingerOverlapping`
  (params (isOverlapping :type Boolean) (Finger :type "/Game/Core/Hand/E_TriggerIndexes Enum" :default "NewEnumerator0") (Actor :type "Actor Object Reference"))
  (`/Engine/EditorBlueprintResources/StandardMacros.IsValid` (`self.GetComponentByClass` Actor "/Game/Blueprints/Components/BPC_GrabComponent.BPC_GrabComponent_C")
    (:`Is Valid`
      (`BlueprintMapLibrary.Map_Add` (`self.FingersOverlapping`) (`local.Finger`) (`local.isOverlapping`))
      (if (`local.isOverlapping`)
        (`BlueprintMapLibrary.Map_Add` (`self.FingersBlocked`) (`local.Finger`) true)))))

(fn `UserConstructionScript`)