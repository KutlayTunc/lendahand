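; Hand Blueprint that curls each finger segment during a grab until it touches the grabbed object, so the fingers conform to its shape.
; StartGrabCurls enables finger collision and plays a timeline whose alpha raises per-segment flex values, freezing each segment on overlap.
; Begin-overlap events accept actors with BPC_GrabComponent, and an 03-segment hit also blocks its 02 segment.
; ClearCurls resets the blocked, overlapping and flex maps.
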(event `self.ReceiveBeginPlay`
  (`self.SetFingerCapsules`))

(event `SetFingerCapsules`
  (set `self.FingersCollisions` (`|MakeMap` "NewEnumerator0" (`self.ColThumb02`) "NewEnumerator2" (`self.ColIndex02`) "NewEnumerator4" (`self.ColMiddle02`) "NewEnumerator6" (`self.ColRing02`) "NewEnumerator8" (`self.ColPinky02`) "NewEnumerator1" (`self.ColThumb03`) "NewEnumerator3" (`self.ColIndex03`) "NewEnumerator5" (`self.ColMiddle03`) "NewEnumerator7" (`self.ColRing03`) "NewEnumerator9" (`self.ColPinky03`) :!type "/Game/Core/Hand/E_TriggerIndexes Enum"))
  (bind _enumvalue (foreach `/Game/Core/Hand/E_TriggerIndexes` false)
    (:`LoopBody`
      (`BlueprintMapLibrary.Map_Add` (`self.FingersBlocked`) _enumvalue)
      (`BlueprintMapLibrary.Map_Add` (`self.FingersFlex`) _enumvalue)
      (`BlueprintMapLibrary.Map_Add` (`self.FingersOverlapping`) _enumvalue))))

(event `StartGrabCurls`
  (params (Actor :type "Actor Object Reference"))
  (set `self.HandAnim` "NewEnumerator1")
  (set `self.GrabActor` Actor)
  (`self.SetCollisionFingers` "QueryAndPhysics")
  (bind (_direction _curltime) (`Timeline|Timeline` :!via `PlayFromStart`)
    (:`Update`
      (`self.EvaluateGrasping` _curltime)
      (`self.HandleCurls` _curltime))))

(event `self.ColThumb02.OnComponentBeginOverlap`
  (params (OverlappedComponent :type "PrimitiveComponent Object Reference") (OtherActor :type "Actor Object Reference") (OtherComp :type "PrimitiveComponent Object Reference") (OtherBodyIndex :type Integer) (bFromSweep :type Boolean) (SweepResult :type "HitResult Structure (by ref)"))
  (`self.SetFingerOverlapping` true "NewEnumerator0" OtherActor))

(event `self.ColIndex02.OnComponentBeginOverlap`
  (params (OverlappedComponent :type "PrimitiveComponent Object Reference") (OtherActor :type "Actor Object Reference") (OtherComp :type "PrimitiveComponent Object Reference") (OtherBodyIndex :type Integer) (bFromSweep :type Boolean) (SweepResult :type "HitResult Structure (by ref)"))
  (`self.SetFingerOverlapping` true "NewEnumerator2" OtherActor))

(event `self.ColMiddle02.OnComponentBeginOverlap`
  (params (OverlappedComponent :type "PrimitiveComponent Object Reference") (OtherActor :type "Actor Object Reference") (OtherComp :type "PrimitiveComponent Object Reference") (OtherBodyIndex :type Integer) (bFromSweep :type Boolean) (SweepResult :type "HitResult Structure (by ref)"))
  (`self.SetFingerOverlapping` true "NewEnumerator4" OtherActor))

(event `self.ColRing02.OnComponentBeginOverlap`
  (params (OverlappedComponent :type "PrimitiveComponent Object Reference") (OtherActor :type "Actor Object Reference") (OtherComp :type "PrimitiveComponent Object Reference") (OtherBodyIndex :type Integer) (bFromSweep :type Boolean) (SweepResult :type "HitResult Structure (by ref)"))
  (`self.SetFingerOverlapping` true "NewEnumerator6" OtherActor))

(event `self.ColPinky02.OnComponentBeginOverlap`
  (params (OverlappedComponent :type "PrimitiveComponent Object Reference") (OtherActor :type "Actor Object Reference") (OtherComp :type "PrimitiveComponent Object Reference") (OtherBodyIndex :type Integer) (bFromSweep :type Boolean) (SweepResult :type "HitResult Structure (by ref)"))
  (`self.SetFingerOverlapping` true "NewEnumerator8" OtherActor))

(event `self.ColThumb03.OnComponentBeginOverlap`
  (params (OverlappedComponent :type "PrimitiveComponent Object Reference") (OtherActor :type "Actor Object Reference") (OtherComp :type "PrimitiveComponent Object Reference") (OtherBodyIndex :type Integer) (bFromSweep :type Boolean) (SweepResult :type "HitResult Structure (by ref)"))
  (`self.SetFingerOverlapping` true "NewEnumerator0" OtherActor)
  (`self.SetFingerOverlapping` true "NewEnumerator1" OtherActor))

(event `self.ColIndex03.OnComponentBeginOverlap`
  (params (OverlappedComponent :type "PrimitiveComponent Object Reference") (OtherActor :type "Actor Object Reference") (OtherComp :type "PrimitiveComponent Object Reference") (OtherBodyIndex :type Integer) (bFromSweep :type Boolean) (SweepResult :type "HitResult Structure (by ref)"))
  (`self.SetFingerOverlapping` true "NewEnumerator2" OtherActor)
  (`self.SetFingerOverlapping` true "NewEnumerator3" OtherActor))

(event `self.ColMiddle03.OnComponentBeginOverlap`
  (params (OverlappedComponent :type "PrimitiveComponent Object Reference") (OtherActor :type "Actor Object Reference") (OtherComp :type "PrimitiveComponent Object Reference") (OtherBodyIndex :type Integer) (bFromSweep :type Boolean) (SweepResult :type "HitResult Structure (by ref)"))
  (`self.SetFingerOverlapping` true "NewEnumerator4" OtherActor)
  (`self.SetFingerOverlapping` true "NewEnumerator5" OtherActor))

(event `self.ColRing03.OnComponentBeginOverlap`
  (params (OverlappedComponent :type "PrimitiveComponent Object Reference") (OtherActor :type "Actor Object Reference") (OtherComp :type "PrimitiveComponent Object Reference") (OtherBodyIndex :type Integer) (bFromSweep :type Boolean) (SweepResult :type "HitResult Structure (by ref)"))
  (`self.SetFingerOverlapping` true "NewEnumerator6" OtherActor)
  (`self.SetFingerOverlapping` true "NewEnumerator7" OtherActor))

(event `self.ColPinky03.OnComponentBeginOverlap`
  (params (OverlappedComponent :type "PrimitiveComponent Object Reference") (OtherActor :type "Actor Object Reference") (OtherComp :type "PrimitiveComponent Object Reference") (OtherBodyIndex :type Integer) (bFromSweep :type Boolean) (SweepResult :type "HitResult Structure (by ref)"))
  (`self.SetFingerOverlapping` true "NewEnumerator8" OtherActor)
  (`self.SetFingerOverlapping` true "NewEnumerator9" OtherActor))

(fn `ClearCurls`
  (locals (ArrElement :type "/Game/Core/Hand/E_TriggerIndexes Enum"))
  (bind _keys (`BlueprintMapLibrary.Map_Keys` (`self.FingersBlocked`)))
  (for _array_element _keys
    (set `local.ArrElement` _array_element)
    (`BlueprintMapLibrary.Map_Add` (`self.FingersBlocked`) (`local.ArrElement`))
    (`BlueprintMapLibrary.Map_Add` (`self.FingersOverlapping`) (`local.ArrElement`))
    (`BlueprintMapLibrary.Map_Add` (`self.FingersFlex`) (`local.ArrElement`))))

(fn `EvaluateGrasping`
  (params (GripAlpha :type "Float (double-precision)"))
  (locals (ArrElement :type "/Game/Core/Hand/E_TriggerIndexes Enum"))
  (bind _keys (`BlueprintMapLibrary.Map_Keys` (`self.FingersCollisions`)))
  (for _array_element _keys
    (set `local.ArrElement` _array_element)
    (if (`BlueprintMapLibrary.Map_Find` (`self.FingersBlocked`) (`local.ArrElement`))
      _
      (elif (`PrimitiveComponent.IsOverlappingActor` (`BlueprintMapLibrary.Map_Find` (`self.FingersCollisions`) (`local.ArrElement`)) (`self.GrabActor`))
        (`BlueprintMapLibrary.Map_Add` (`self.FingersOverlapping`) (`local.ArrElement`) true)
        (`BlueprintMapLibrary.Map_Add` (`self.FingersBlocked`) (`local.ArrElement`) true)
        (else
          (`self.FingerMovement` (`local.ArrElement`) (`local.GripAlpha`)))))))

(fn `FingerMovement`
  (params (FingerIndex :type "/Game/Core/Hand/E_TriggerIndexes Enum" :default "NewEnumerator0") (AlphaInput :type "Float (double-precision)"))
  (if (> (`KismetMathLibrary.Abs` (- (`local.AlphaInput`) (`BlueprintMapLibrary.Map_Find` (`self.FingersFlex`) (`local.FingerIndex`)))) 0.05)
    (`BlueprintMapLibrary.Map_Add` (`self.FingersFlex`) (`local.FingerIndex`) (`local.AlphaInput`))))

(fn `HandleCurls`
  (params (GripAlpha :type "Float (double-precision)"))
  (locals (ArrElement :type "/Game/Core/Hand/E_TriggerIndexes Enum"))
  (bind _keys (`BlueprintMapLibrary.Map_Keys` (`self.FingersBlocked`)))
  (for _array_element _keys
    (set `local.ArrElement` _array_element)
    (if (> (`local.GripAlpha`) (`BlueprintMapLibrary.Map_Find` (`self.FingersFlex`) (`local.ArrElement`)))
      _
      (elif (`BlueprintMapLibrary.Map_Find` (`self.FingersBlocked`) (`local.ArrElement`))
        (if (or (< (`local.GripAlpha`) (`BlueprintMapLibrary.Map_Find` (`self.FingersFlex`) (`local.ArrElement`))) (not (`BlueprintMapLibrary.Map_Find` (`self.FingersOverlapping`) (`local.ArrElement`))))
          (`BlueprintMapLibrary.Map_Add` (`self.FingersBlocked`) (`local.ArrElement`))
          (`self.FingerMovement` (`local.ArrElement`) (`local.GripAlpha`)))
        (else
          (`self.FingerMovement` (`local.ArrElement`) (`local.GripAlpha`)))))))

(fn `SetCollisionFingers`
  (params (NewParam :type "ECollisionEnabled Enum" :default "NoCollision"))
  (for _array_element (`|MakeArray` (`self.ColMiddle03`) (`self.ColIndex02`) (`self.ColMiddle02`) (`self.ColRing02`) (`self.ColPinky02`) (`self.ColThumb02`) (`self.ColThumb03`) (`self.ColIndex03`) (`self.ColRing03`) (`self.ColPinky03`))
    (`PrimitiveComponent.SetCollisionEnabled` _array_element NewParam)))

(fn `SetFingerOverlapping`
  (params (isOverlapping :type Boolean) (Finger :type "/Game/Core/Hand/E_TriggerIndexes Enum" :default "NewEnumerator0") (Actor :type "Actor Object Reference"))
  (`/Engine/EditorBlueprintResources/StandardMacros.IsValid` (`self.GetComponentByClass` Actor "/Game/Blueprints/Components/BPC_GrabComponent.BPC_GrabComponent_C")
    (:`Is Valid`
      (`BlueprintMapLibrary.Map_Add` (`self.FingersOverlapping`) (`local.Finger`) (`local.isOverlapping`))
      (if (`local.isOverlapping`)
        (`BlueprintMapLibrary.Map_Add` (`self.FingersBlocked`) (`local.Finger`) true)))))

(fn `UserConstructionScript`)