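; Hand helper component for BP_MotionController that eases the hand mesh toward nearby grabbable objects.
; StartOverlapTimer runs a per-frame loop that finds the closest BP_Grabbable and grab component in the proximity sphere, caching its GrabProfile, until none overlap.
; For Side grabs, it rotates the grab point around the object in mesh space to follow the controller, blending hand position by distance.
; UpdateHandPose is a stub, and surface-touch logic is unwired.
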(event `self.ReceiveBeginPlay`
  (bind _asbp_motion_controller (cast `/Game/Core/Character/BP_MotionController` (`self.GetOwner`)))
  (set `self.Motion Controller` (`/Game/Core/Character/BP_MotionController.MotionController` _asbp_motion_controller))
  (set `self.Skeletal Mesh` (`/Game/Core/Character/BP_MotionController.HandMesh` _asbp_motion_controller))
  (set `self.Proximity Sphere` (`/Game/Core/Character/BP_MotionController.ProximitySphere` _asbp_motion_controller)))

(event `StartOverlapTimer`
  (bind _returnvalue (`KismetSystemLibrary.K2_SetTimerDelegate` (delegate `CheckClosestActorOnOverlap`) (`GameplayStatics.GetWorldDeltaSeconds`) true))
  (set `self.OverlapTimerHandle` _returnvalue))

(event `CheckClosestActorOnOverlap`
  (`self.FindClosestActorAndGrabComponent`)
  (`self.ReachToClosestGrabComponent`)
  (`self.UpdateHandPose`))

(fn `FindClosestActorAndGrabComponent`
  (locals (OverlappedActor :type "Actor Object Reference") (GrabComponent :type "/Game/Core/Grabbable/BPC_GrabComponent Object Reference") (DistanceOverlappedActor :type "Float (double-precision)" :default 10000.0) (DistanceOverlappedGrabComponent :type "Float (double-precision)" :default 10000.0))
  (bind _overlappingactors (`PrimitiveComponent.GetOverlappingActors` (`self.Proximity Sphere`) "/Game/Core/Grabbable/BP_Grabbable.BP_Grabbable_C"))
  (bind _returnvalue (`KismetMathLibrary.VSizeSquared` (- (`SceneComponent.K2_GetComponentLocation` (`self.Motion Controller`)) (`SceneComponent.K2_GetComponentLocation` (`local.GrabComponent`)))))
  (bind _returnvalue_2 (`KismetMathLibrary.VSizeSquared` (- (`Actor.K2_GetActorLocation` (`local.OverlappedActor`)) (`SceneComponent.K2_GetComponentLocation` (`self.Motion Controller`)))))
  (if (> (`KismetArrayLibrary.Array_Length` _overlappingactors) 0)
    (for _array_element _overlappingactors
      (set `local.OverlappedActor` _array_element)
      (if (<= _returnvalue_2 (`local.DistanceOverlappedActor`))
        (set `local.DistanceOverlappedActor` _returnvalue_2)
        (`|ExecutionSequence`
          (:`then_0`
            (if (!= (`local.OverlappedActor`) (`self.ClosestActorOnOverlap`))
              (set `self.ClosestActorOnOverlap` (`local.OverlappedActor`))))
          (:`then_1`
            (bind _closestactoronoverlap (`self.ClosestActorOnOverlap`)
              (:`then`
                (for _array_element_2 (`Actor.K2_GetComponentsByClass` _closestactoronoverlap "/Game/Core/Grabbable/BPC_GrabComponent.BPC_GrabComponent_C")
                  (set `local.GrabComponent` _array_element_2)
                  (if (<= _returnvalue (`local.DistanceOverlappedGrabComponent`))
                    (set `local.DistanceOverlappedGrabComponent` _returnvalue)
                    (if (!= (`local.GrabComponent`) (`self.ClosestGrabComponentOnOverlap`))
                      (set `self.ClosestGrabComponentOnOverlap` (`local.GrabComponent`))
                      (`self.SetGrabProfileOnOverlap`))))
                (set `local.DistanceOverlappedGrabComponent` 10000.0))
              (:`else`))))))
    (set `local.DistanceOverlappedActor` 10000.0)
    (else
      (`KismetSystemLibrary.K2_ClearAndInvalidateTimerHandle` (`self.OverlapTimerHandle`))
      (set `self.ClosestActorOnOverlap` null)
      (set `local.DistanceOverlappedActor` 10000.0)
      (set `local.DistanceOverlappedGrabComponent` 10000.0))))

(fn `ReachToClosestGrabComponent`
  (locals (MotionControllerLocationWS :type "Vector Structure" :default (0.0 0.0 0.0)) (MotionControllerLocationMS :type "Vector Structure" :default (0.0 0.0 0.0)) (MeshCenterLocationMS :type "Vector Structure" :default (0.0 0.0 0.0)) (MeshWorldTransform :type "Transform Structure") (GrabPointLocationMS :type "Vector Structure" :default (0.0 0.0 0.0)) (AngleBetweenMotionControllerAndGrabPoint :type "Float (double-precision)" :default 0.0) (DistanceAdjustMultiplier :type "Float (double-precision)"))
  (bind (_grabpointlocationms_x _grabpointlocationms_y) (`KismetMathLibrary.BreakVector` (`local.GrabPointLocationMS`)))
  (bind _closestgrabcomponentonoverlap (`self.ClosestGrabComponentOnOverlap`))
  (bind (_motioncontrollerlocationms_x _motioncontrollerlocationms_y) (`KismetMathLibrary.BreakVector` (`local.MotionControllerLocationMS`)))
  (bind (_grabpointlocationms_x_2 _grabpointlocationms_y_2 _grabpointlocationms_z) (`KismetMathLibrary.BreakVector` (`local.GrabPointLocationMS`)))
  (bind (_meshcenterlocationms_x _meshcenterlocationms_y) (`KismetMathLibrary.BreakVector` (`local.MeshCenterLocationMS`)))
  (bind (_motioncontrollerlocationms_x_2 _motioncontrollerlocationms_y_2 _motioncontrollerlocationms_z) (`KismetMathLibrary.BreakVector` (`local.MotionControllerLocationMS`)))
  (bind (_grabprofile_proptype _grabprofile_grabdirection) (break `/Game/Core/Grabbable/Structs/S_GrabProfile` (`self.GrabProfile`)))
  (bind _returnvalue (`KismetMathLibrary.Normal` (`KismetMathLibrary.MakeVector` _motioncontrollerlocationms_x _motioncontrollerlocationms_y)))
  (bind _returnvalue_2 (`KismetMathLibrary.Normal` (`KismetMathLibrary.MakeVector` _grabpointlocationms_x _grabpointlocationms_y)))
  (bind _returnvalue_3 (`SceneComponent.GetAttachParent` _closestgrabcomponentonoverlap))
  (bind _returnvalue_4 (`SceneComponent.K2_GetComponentLocation` (`self.Motion Controller`)))
  (bind (_returnvalue_x _returnvalue_y _returnvalue_z) (`KismetMathLibrary.BreakVector` (`KismetMathLibrary.Cross_VectorVector` _returnvalue_2 _returnvalue)))
  (bind _returnvalue_5 (`KismetMathLibrary.MapRangeClamped` (`KismetMathLibrary.Vector_Distance` _returnvalue_4 (`self.ClosestGrabComponentDynamicLocation`)) 0.0 (`SphereComponent.SphereRadius` (`self.Proximity Sphere`)) 0.0 1.0))
  (switch `/Game/Core/Grabbable/Enums/E_GrabDirection` _grabprofile_grabdirection
    (:`NewEnumerator1`
      ;[0.05161 0.1165 0.15 0.5] Variables Set
      (set `local.MotionControllerLocationWS` (`SceneComponent.K2_GetComponentLocation` (`self.Motion Controller`)))
      (set `local.GrabPointLocationMS` (`SceneComponent.RelativeLocation` _closestgrabcomponentonoverlap))
      (set `local.MeshCenterLocationMS` (`SceneComponent.RelativeLocation` _returnvalue_3))
      (set `local.MeshWorldTransform` (`SceneComponent.K2_GetComponentToWorld` _returnvalue_3))
      (set `local.MotionControllerLocationMS` (`KismetMathLibrary.InverseTransformLocation` (`local.MeshWorldTransform`) (`local.MotionControllerLocationWS`)))
      ;[0.15 0.1284 0.08458 0.5] Angle Between Motion Controller and Grab Poin in MESH SPACE
      (bind _output_get (set `local.AngleBetweenMotionControllerAndGrabPoint` (mod (+ (`KismetMathLibrary.DegAtan2` _returnvalue_z (`KismetMathLibrary.Dot_VectorVector` _returnvalue_2 _returnvalue)) 360.0) 360.0)))
      (bind (_returnvalue_x_2 _returnvalue_y_2) (`KismetMathLibrary.BreakVector` (`KismetMathLibrary.RotateAngleAxis` (`KismetMathLibrary.MakeVector` _grabpointlocationms_x_2 _grabpointlocationms_y_2 _grabpointlocationms_z) _output_get (`KismetMathLibrary.MakeVector` _meshcenterlocationms_x _meshcenterlocationms_y _grabpointlocationms_z))))
      ;[0.15 0.124 0.08406 0.5] Reach Hand To Object Based on Hand Distance
      (bind _output_get_2 (set `self.ClosestGrabComponentDynamicLocation` (`KismetMathLibrary.TransformLocation` (`local.MeshWorldTransform`) (`KismetMathLibrary.MakeVector` _returnvalue_x_2 _returnvalue_y_2 _motioncontrollerlocationms_z))))
      (set `self.HandDistanceAlpha` _returnvalue_5)
      (`SceneComponent.K2_SetWorldLocation` (`self.Skeletal Mesh`) (+ _output_get_2 (* (* (`KismetMathLibrary.GetDirectionUnitVector` _output_get_2 _returnvalue_4) _returnvalue_5) (* _returnvalue_5 (`SphereComponent.SphereRadius` (`self.Proximity Sphere`))))) false false)
      ;[0.111 0.08701 0.15 0.5] Rotate Hand To Obj
      (`SceneComponent.K2_SetWorldRotation` (`self.Skeletal Mesh`) (`KismetMathLibrary.RInterpTo` (`SceneComponent.K2_GetComponentRotation` (`self.Skeletal Mesh`)) (`KismetMathLibrary.TransformRotation` (`local.MeshWorldTransform`) (`KismetMathLibrary.ComposeRotators` (`SceneComponent.RelativeRotation` (`self.ClosestGrabComponentOnOverlap`)) (`KismetMathLibrary.MakeRotator` 0.0 0.0 (`local.AngleBetweenMotionControllerAndGrabPoint`)))) (`GameplayStatics.GetWorldDeltaSeconds`) 25.0) false false))))

(fn `SetGrabProfileOnOverlap`
  (bind _closestgrabcomponentonoverlap (`self.ClosestGrabComponentOnOverlap`)
    (:`then`
      (bind _asbpc_grab_component (cast `/Game/Core/Grabbable/BPC_GrabComponent` _closestgrabcomponentonoverlap))
      (set `self.GrabProfile` (`/Game/Core/Grabbable/BPC_GrabComponent.GrabProfile` _asbpc_grab_component)))
    (:`else`)))

(fn `UpdateHandPose`
  (bind (_grabprofile_proptype _grabprofile_grabdirection _grabprofile_animation _grabprofile_overlapbehaviour) (break `/Game/Core/Grabbable/Structs/S_GrabProfile` (`self.GrabProfile`)))
  (switch `/Game/Core/Grabbable/Enums/E_OverlapBehaviour` _grabprofile_overlapbehaviour))