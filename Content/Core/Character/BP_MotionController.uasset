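; BP_MotionController is a VR hand Blueprint with a motion controller, hand mesh and proximity sphere.
; Construction sets the motion source from the Hand enum, orients the mesh and mirrors it on Z for the left hand.
; Sphere overlaps start an overlap timer on BPCHandHelper.
; On BeginPlay, a timeline prints its value each update and calls TryGrab on that helper when finished, which looks like test scaffolding.
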(event `self.ReceiveBeginPlay`
  (bind (_direction _newtrack_0) (`Timeline|Timeline` :!via `PlayFromStart`)
    (:`Update`
      (`KismetSystemLibrary.PrintString` (`KismetStringLibrary.Conv_DoubleToString` _newtrack_0) true true (struct :`G` 0.66 :`B` 1.0 :`A` 1.0) (`GameplayStatics.GetWorldDeltaSeconds`)))
    (:`Finished`
      (`/Game/Core/Character/BPC_HandHelper.TryGrab` (`self.BPC_HandHelper`)))))

(event `self.ProximitySphere.OnComponentBeginOverlap`
  (params (OverlappedComponent :type "PrimitiveComponent Object Reference") (OtherActor :type "Actor Object Reference") (OtherComp :type "PrimitiveComponent Object Reference") (OtherBodyIndex :type Integer) (bFromSweep :type Boolean) (SweepResult :type "HitResult Structure (by ref)"))
  (`/Game/Core/Character/BPC_HandHelper.StartOverlapTimer` (`self.BPC_HandHelper`)))

(event `self.ProximitySphere.OnComponentEndOverlap`
  (params (OverlappedComponent :type "PrimitiveComponent Object Reference") (OtherActor :type "Actor Object Reference") (OtherComp :type "PrimitiveComponent Object Reference") (OtherBodyIndex :type Integer)))

(fn `UserConstructionScript`
  (`SceneComponent.K2_SetRelativeRotation` (`self.HandMesh`) (struct :`Pitch` 120.0 :`Roll` 90.0) false false)
  (set `MotionControllerComponent.MotionSource` (`|GetEnumeratorName` (`self.Hand`)) (`self.MotionController`))
  (switch `EControllerHand` (`self.Hand`)
    (:`Left`
      (`SceneComponent.SetWorldScale3D` (`self.HandMesh`) (1.0 1.0 -1.0)))))