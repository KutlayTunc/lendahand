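; VR hand component for BP_MotionController that snaps the hand mesh toward nearby grab points.
; A per-frame timer, started on overlap, finds the closest BP_Grabbable in the proximity sphere and its closest BPC_GrabComponent, stopping when none overlap.
; For Side grab profiles, it works in the grabbable's mesh space, swinging the grab point by the controller's angle and matching its height, so the hand slides around the object.
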(event `self.ReceiveBeginPlay`
  (bind _asbp_motion_controller (cast `/Game/Core/Character/BP_MotionController` (`self.GetOwner`)))
  (set `self.Motion Controller` (`/Game/Core/Character/BP_MotionController.MotionController` _asbp_motion_controller))
  (set `self.Skeletal Mesh` (`/Game/Core/Character/BP_MotionController.HandMesh` _asbp_motion_controller))
  (set `self.Proximity Sphere` (`/Game/Core/Character/BP_MotionController.ProximitySphere` _asbp_motion_controller)))

(event `StartTimerOnOverlap`
  (bind _returnvalue (`KismetSystemLibrary.K2_SetTimerDelegate` (delegate `StartCheckClosestActorOnOverlap`) (`GameplayStatics.GetWorldDeltaSeconds`) true))
  (set `self.ClosestActorCheckTimer` _returnvalue))

(event `StartCheckClosestActorOnOverlap`
  (`self.SetClosestActorAndGrabComponentOnOverlap`)
  (`self.HandReachClosestGrabPoint`))

(fn `HandReachClosestGrabPoint`
  (locals (MotionControllerLocationWS :type "Vector Structure" :default (0.0 0.0 0.0)) (MotionControllerLocationMS :type "Vector Structure" :default (0.0 0.0 0.0)) (MeshCenterLocationMS :type "Vector Structure" :default (0.0 0.0 0.0)) (MeshWorldTransform :type "Transform Structure") (OrbitOffset :type "Vector Structure") (GrabPointLocationMS :type "Vector Structure" :default (0.0 0.0 0.0)) (NewLocalVar :type "Vector Structure" :default (0.0 0.0 0.0)) (AngleBetweenMotionControllerAndGrabPoint :type "Float (double-precision)" :default 0.0))
  (bind (_grabpointlocationms_x _grabpointlocationms_y) (`KismetMathLibrary.BreakVector` (`local.GrabPointLocationMS`)))
  (bind _closestgrabcomponentonoverlap (`self.ClosestGrabComponentOnOverlap`))
  (bind (_motioncontrollerlocationms_x _motioncontrollerlocationms_y) (`KismetMathLibrary.BreakVector` (`local.MotionControllerLocationMS`)))
  (bind (_grabpointlocationms_x_2 _grabpointlocationms_y_2 _grabpointlocationms_z) (`KismetMathLibrary.BreakVector` (`local.GrabPointLocationMS`)))
  (bind (_meshcenterlocationms_x _meshcenterlocationms_y) (`KismetMathLibrary.BreakVector` (`local.MeshCenterLocationMS`)))
  (bind (_motioncontrollerlocationms_x_2 _motioncontrollerlocationms_y_2 _motioncontrollerlocationms_z) (`KismetMathLibrary.BreakVector` (`local.MotionControllerLocationMS`)))
  (bind _returnvalue (`KismetMathLibrary.Normal` (`KismetMathLibrary.MakeVector` _motioncontrollerlocationms_x _motioncontrollerlocationms_y)))
  (bind _returnvalue_2 (`KismetMathLibrary.Normal` (`KismetMathLibrary.MakeVector` _grabpointlocationms_x _grabpointlocationms_y)))
  (bind _returnvalue_3 (`SceneComponent.GetAttachParent` _closestgrabcomponentonoverlap))
  (bind (_returnvalue_x _returnvalue_y _returnvalue_z) (`KismetMathLibrary.BreakVector` (`KismetMathLibrary.Cross_VectorVector` _returnvalue_2 _returnvalue)))
  (bind _closestgrabcomponentonoverlap_2 (`self.ClosestGrabComponentOnOverlap`)
    (:`then`
      (bind _asbpc_grab_component (cast `/Game/Core/Grabbable/BPC_GrabComponent` _closestgrabcomponentonoverlap_2))
      (bind (_grabprofile_proptype _grabprofile_grablocation) (break `/Game/Core/Grabbable/Structs/S_GrabProfile` (`/Game/Core/Grabbable/BPC_GrabComponent.GrabProfile` _asbpc_grab_component)))
      (switch `/Game/Core/Grabbable/Enums/E_GrabLocation` _grabprofile_grablocation
        (:`NewEnumerator1`
          (set `local.MotionControllerLocationWS` (`SceneComponent.K2_GetComponentLocation` (`self.Motion Controller`)))
          (set `local.GrabPointLocationMS` (`SceneComponent.RelativeLocation` _closestgrabcomponentonoverlap))
          (set `local.MeshCenterLocationMS` (`SceneComponent.RelativeLocation` _returnvalue_3))
          (set `local.MeshWorldTransform` (`SceneComponent.K2_GetComponentToWorld` _returnvalue_3))
          (set `local.MotionControllerLocationMS` (`KismetMathLibrary.InverseTransformLocation` (`local.MeshWorldTransform`) (`local.MotionControllerLocationWS`)))
          ; Angle Between Motion Controller and Grab Poin in MESH SPACE
          (bind _output_get (set `local.AngleBetweenMotionControllerAndGrabPoint` (mod (+ (`KismetMathLibrary.DegAtan2` _returnvalue_z (`KismetMathLibrary.Dot_VectorVector` _returnvalue_2 _returnvalue)) 360.0) 360.0)))
          (bind (_returnvalue_x_2 _returnvalue_y_2) (`KismetMathLibrary.BreakVector` (`KismetMathLibrary.RotateAngleAxis` (`KismetMathLibrary.MakeVector` _grabpointlocationms_x_2 _grabpointlocationms_y_2 _grabpointlocationms_z) _output_get (`KismetMathLibrary.MakeVector` _meshcenterlocationms_x _meshcenterlocationms_y _grabpointlocationms_z))))
          (`SceneComponent.K2_SetWorldLocation` (`self.Skeletal Mesh`) (`KismetMathLibrary.TransformLocation` (`local.MeshWorldTransform`) (`KismetMathLibrary.MakeVector` _returnvalue_x_2 _returnvalue_y_2 _motioncontrollerlocationms_z)) false false)
          (`SceneComponent.K2_SetWorldRotation` (`self.Skeletal Mesh`) (`KismetMathLibrary.TransformRotation` (`local.MeshWorldTransform`) (`KismetMathLibrary.ComposeRotators` (`SceneComponent.RelativeRotation` (`self.ClosestGrabComponentOnOverlap`)) (`KismetMathLibrary.MakeRotator` 0.0 0.0 (- (`local.AngleBetweenMotionControllerAndGrabPoint`) 360.0)))) false false))))
    (:`else`)))

(fn `SetClosestActorAndGrabComponentOnOverlap`
  (locals (OverlappedActor :type "Actor Object Reference") (GrabComponent :type "/Game/Core/Grabbable/BPC_GrabComponent Object Reference") (DistanceOverlappedActor :type "Float (double-precision)" :default 10000.0) (DistanceOverlappedGrabComponent :type "Float (double-precision)" :default 10000.0))
  (bind _overlappingactors (`PrimitiveComponent.GetOverlappingActors` (`self.Proximity Sphere`) "/Game/Core/Grabbable/BP_Grabbable.BP_Grabbable_C"))
  (bind _returnvalue (`KismetMathLibrary.VSizeSquared` (- (`SceneComponent.K2_GetComponentLocation` (`self.Motion Controller`)) (`SceneComponent.K2_GetComponentLocation` (`local.GrabComponent`)))))
  (bind _returnvalue_2 (`KismetMathLibrary.VSizeSquared` (- (`Actor.K2_GetActorLocation` (`local.OverlappedActor`)) (`SceneComponent.K2_GetComponentLocation` (`self.Motion Controller`)))))
  (if (> (`KismetArrayLibrary.Array_Length` _overlappingactors) 0)
    (for _array_element _overlappingactors
      (set `local.OverlappedActor` _array_element)
      (if (<= _returnvalue_2 (`local.DistanceOverlappedActor`))
        (set `local.DistanceOverlappedActor` _returnvalue_2)
        (`|ExecutionSequence`
          (:`then_0`
            (if (!= (`local.OverlappedActor`) (`self.ClosestActorOnOverlap`))
              (set `self.ClosestActorOnOverlap` (`local.OverlappedActor`))))
          (:`then_1`
            (bind _closestactoronoverlap (`self.ClosestActorOnOverlap`)
              (:`then`
                (for _array_element_2 (`Actor.K2_GetComponentsByClass` _closestactoronoverlap "/Game/Core/Grabbable/BPC_GrabComponent.BPC_GrabComponent_C")
                  (set `local.GrabComponent` _array_element_2)
                  (if (<= _returnvalue (`local.DistanceOverlappedGrabComponent`))
                    (set `local.DistanceOverlappedGrabComponent` _returnvalue)
                    (if (!= (`local.GrabComponent`) (`self.ClosestGrabComponentOnOverlap`))
                      (set `self.ClosestGrabComponentOnOverlap` (`local.GrabComponent`)))))
                (set `local.DistanceOverlappedGrabComponent` 10000.0))
              (:`else`))))))
    (set `local.DistanceOverlappedActor` 10000.0)
    (else
      (`KismetSystemLibrary.K2_ClearAndInvalidateTimerHandle` (`self.ClosestActorCheckTimer`))
      (set `self.ClosestActorOnOverlap` null)
      (set `local.DistanceOverlappedActor` 10000.0)
      (set `local.DistanceOverlappedGrabComponent` 10000.0))))