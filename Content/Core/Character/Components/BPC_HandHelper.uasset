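; VR hand component for BP_MotionController that drives a physics-controlled hand mesh toward nearby BP_Grabbable objects.
; A looping overlap timer finds the closest grabbable and grab component, then eases the hand toward it by controller distance.
; Side grabs rotate the grab point around the object to face the controller, mirrored for left hands.
; TryGrab is empty, leaving the timed snap-and-attach grab unreached; surface-touch logic is also disconnected.
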(event `self.ReceiveBeginPlay`
  ;[0.15 0.08828 0.08828 0.5 20] BeginPlay
  (`self.SetValues`)
  (`self.SetPhysicsControl`))

(event `StartOverlapTimer`
  (params (Actor :type "Actor Object Reference"))
  ; Overlap Timer
  (`self.SetInitialHandDistance` Actor)
  (bind _returnvalue (`KismetSystemLibrary.K2_SetTimerDelegate` (delegate `OverlapTimerEvent`) (`GameplayStatics.GetWorldDeltaSeconds`) true true))
  (set `self.OverlapTimerHandle` _returnvalue))

(event `OverlapTimerEvent`
  ; Overlap Timer
  (`KismetSystemLibrary.PrintString` "OverlapTimer" true true (struct :`G` 0.66 :`B` 1.0 :`A` 1.0) 2.0 "overlaptimer")
  (`self.ClearValuesIfOverlapEmpty`)
  (`self.FindClosestActor`)
  (`self.FindClosestGrabComponent`)
  (`self.SetGrabProfile`)
  (`self.ReachToClosestGrabComponent`))

(event `TryGrab`
  ; Grab Timer
)

(event `GrabTimerEvent`
  ; Grab Timer
  (`KismetSystemLibrary.PrintString` "grabtimer" true true (struct :`G` 0.66 :`B` 1.0 :`A` 1.0) 2.0 "grabtimer")
  (`self.FindClosestActor`)
  (`self.FindClosestGrabComponent`)
  (bind _final (`self.FinalizeHandReach`))
  (if _final
    (`KismetSystemLibrary.K2_ClearAndInvalidateTimerHandle` (`self.GrabTimerHandle`))
    (bind _asbp_grabbable (cast `/Game/Core/Grabbable/BP_Grabbable` (`self.ClosestActorOnOverlap`)))
    (`SceneComponent.K2_AttachToComponent` (`/Game/Core/Grabbable/BP_Grabbable.StaticMesh` _asbp_grabbable) (`self.Skeletal Mesh`) "None" "KeepWorld" "KeepWorld" "KeepWorld" false)
    (`PrimitiveComponent.SetSimulatePhysics` (`self.Skeletal Mesh`) true)
    (set `self.GrabbedActor` (`self.ClosestActorOnOverlap`))))

(event `TryRelease`
  (`KismetSystemLibrary.PrintString` (`KismetStringLibrary.Concat_StrStr` "BPCHandHelper-" (`|GetEnumeratorNameAsString` (`self.Hand`)) "-TryRelease") true true (struct :`R` 1.0 :`G` 0.514862 :`A` 1.0) 2.0 "line")
  (`KismetSystemLibrary.K2_ClearAndInvalidateTimerHandle` (`self.GrabTimerHandle`))
  (bind _asbp_grabbable (cast `/Game/Core/Grabbable/BP_Grabbable` (`self.GrabbedActor`)))
  (`PrimitiveComponent.SetSimulatePhysics` (`/Game/Core/Grabbable/BP_Grabbable.StaticMesh` _asbp_grabbable) true))

(fn `ClearValuesIfOverlapEmpty`
  (if (<= (`KismetArrayLibrary.Array_Length` (`PrimitiveComponent.GetOverlappingActors` (`self.Proximity Sphere`) "/Game/Core/Grabbable/BP_Grabbable.BP_Grabbable_C")) 0)
    (`KismetSystemLibrary.K2_ClearAndInvalidateTimerHandle` (`self.OverlapTimerHandle`))
    (set `self.ClosestActorOnOverlap` null)
    (set `self.ClosestGrabComponentOnOverlap` null)
    (`self.SetHandAnimState` "NewEnumerator0")
    (`PrimitiveComponent.SetSimulatePhysics` (`self.Skeletal Mesh`) true)
    (`PrimitiveComponent.SetCollisionEnabled` (`self.Skeletal Mesh`) "QueryAndPhysics")
    (set `self.ElapsedTime` 0.0)))

(fn `FinalizeHandReach`
  (returns (Final :type Boolean))
  (`self.ClosestGrabComponentOnOverlap`
    (:`then`
      (`SceneComponent.K2_SetWorldLocation` (`self.Skeletal Mesh`) (`KismetMathLibrary.VLerp` (`SceneComponent.K2_GetComponentLocation` (`self.Skeletal Mesh`)) (`KismetMathLibrary.TransformLocation` (`SceneComponent.K2_GetComponentToWorld` (`SceneComponent.GetAttachParent` (`self.ClosestGrabComponentOnOverlap`))) (`self.AdjustedGrabPointLocationMS`)) (`self.GetAcceleratedAlpha`)) false false)
      (`SceneComponent.K2_SetWorldRotation` (`self.Skeletal Mesh`) (`KismetMathLibrary.RLerp` (`SceneComponent.K2_GetComponentRotation` (`self.Skeletal Mesh`)) (`KismetMathLibrary.TransformRotation` (`SceneComponent.K2_GetComponentToWorld` (`SceneComponent.GetAttachParent` (`self.ClosestGrabComponentOnOverlap`))) (`self.AdjustedGrabPointRotation`)) (`self.GetAcceleratedAlpha`) true) false false)
      (set `self.HandDistanceAlpha` (`KismetMathLibrary.MapRangeClamped` (`KismetMathLibrary.Vector_Distance` (`SceneComponent.K2_GetComponentLocation` (`self.Skeletal Mesh`)) (`self.AdjustedClosestGrabPointWS`)) (`self.InitialHandToMeshDistance`) 0.0 (`self.HandDistanceAlpha`) 1.0))
      (if (>= (`self.GetAcceleratedAlpha`) 1.0)
        (`SceneComponent.K2_SetWorldLocation` (`self.Skeletal Mesh`) (`KismetMathLibrary.TransformLocation` (`SceneComponent.K2_GetComponentToWorld` (`SceneComponent.GetAttachParent` (`self.ClosestGrabComponentOnOverlap`))) (`self.AdjustedGrabPointLocationMS`)) false false)
        (`SceneComponent.K2_SetWorldRotation` (`self.Skeletal Mesh`) (`KismetMathLibrary.TransformRotation` (`SceneComponent.K2_GetComponentToWorld` (`SceneComponent.GetAttachParent` (`self.ClosestGrabComponentOnOverlap`))) (`self.AdjustedGrabPointRotation`)) false false)
        (return true)
        (else
          (return false))))
    (:`else`)))

(fn `FindClosestActor`
  (locals (OverlappedActor :type "Actor Object Reference") (GrabComponent :type "/Game/Core/Grabbable/BPC_GrabComponent Object Reference") (DistanceOverlappedActor :type "Float (double-precision)" :default 10000.0) (DistanceOverlappedGrabComponent :type "Float (double-precision)" :default 10000.0))
  (bind _overlappingactors (`PrimitiveComponent.GetOverlappingActors` (`self.Proximity Sphere`) "/Game/Core/Grabbable/BP_Grabbable.BP_Grabbable_C"))
  (bind _returnvalue (`KismetMathLibrary.VSizeSquared` (- (`Actor.K2_GetActorLocation` (`local.OverlappedActor`)) (`SceneComponent.K2_GetComponentLocation` (`self.Motion Controller`)))))
  (if (> (`KismetArrayLibrary.Array_Length` _overlappingactors) 0)
    (for _array_element _overlappingactors
      (set `local.OverlappedActor` _array_element)
      (if (<= _returnvalue (`local.DistanceOverlappedActor`))
        (set `local.DistanceOverlappedActor` _returnvalue)
        (if (!= (`local.OverlappedActor`) (`self.ClosestActorOnOverlap`))
          (set `self.ClosestActorOnOverlap` (`local.OverlappedActor`))
          (`self.SetHandAnimState` "NewEnumerator1"))))
    (set `local.DistanceOverlappedActor` 10000.0)
    (else
      (set `local.DistanceOverlappedActor` 10000.0))))

(fn `FindClosestGrabComponent`
  (locals (GrabComponent :type "/Game/Core/Grabbable/BPC_GrabComponent Object Reference") (DistanceOverlappedGrabComponent :type "Float (double-precision)" :default 10000.0))
  (bind _returnvalue (`KismetMathLibrary.VSizeSquared` (- (`SceneComponent.K2_GetComponentLocation` (`self.Motion Controller`)) (`SceneComponent.K2_GetComponentLocation` (`local.GrabComponent`)))))
  (bind _closestactoronoverlap (`self.ClosestActorOnOverlap`)
    (:`then`
      (bind _returnvalue_2 (`Actor.K2_GetComponentsByClass` _closestactoronoverlap "/Game/Core/Grabbable/BPC_GrabComponent.BPC_GrabComponent_C"))
      (if (> (`KismetArrayLibrary.Array_Length` _returnvalue_2) 0)
        (for _array_element _returnvalue_2
          (set `local.GrabComponent` _array_element)
          (if (<= _returnvalue (`local.DistanceOverlappedGrabComponent`))
            (set `local.DistanceOverlappedGrabComponent` _returnvalue)
            (set `self.ClosestGrabComponentOnOverlap` (`local.GrabComponent`))))
        (set `local.DistanceOverlappedGrabComponent` 10000.0)
        (else
          (set `local.DistanceOverlappedGrabComponent` 10000.0)
          (set `self.ClosestGrabComponentOnOverlap` null))))
    (:`else`)))

(fn `GetAcceleratedAlpha`
  (returns (ElapsedTimeAlpha :type "Float (double-precision)"))
  (bind _output_get (set `self.ElapsedTime` (+ (* (`self.ElapsedTimeSpeedMultiplier`) (`GameplayStatics.GetWorldDeltaSeconds`)) (`self.ElapsedTime`))))
  (return _output_get))

(fn `HandleHandsOnTeleport`
  (params (Simulate :type Boolean))
  (`PrimitiveComponent.SetSimulatePhysics` (`self.Skeletal Mesh`) (`local.Simulate`))
  (`SceneComponent.K2_AttachToComponent` (`self.Skeletal Mesh`) (`self.Anchor`) "None" "KeepWorld" "KeepWorld" "KeepWorld" false))

(fn `ReachToClosestGrabComponent`
  (locals (MotionControllerLocationWS :type "Vector Structure" :default (0.0 0.0 0.0)) (MotionControllerLocationMS :type "Vector Structure" :default (0.0 0.0 0.0)) (MeshCenterLocationMS :type "Vector Structure" :default (0.0 0.0 0.0)) (MeshWorldTransform :type "Transform Structure") (GrabPointLocationMS :type "Vector Structure" :default (0.0 0.0 0.0)) (AngleBetweenMotionControllerAndGrabPoint :type "Float (double-precision)" :default 0.0) (MotionControllerLocationWS :type "Vector Structure") (GrabPointLocationMS :type "Vector Structure") (MeshCenterLocationMS :type "Vector Structure") (MeshWorldTransform :type "Transform Structure") (MotionControllerLocationMS :type "Vector Structure") (AngleBetweenMotionControllerAndGrabPoint :type "Float (double-precision)") (Distance :type "Float (double-precision)" :default 0.0) (UnitDirectionFromGrabToMC :type "Vector Structure" :default (0.0 0.0 0.0)))
  (bind (_grabpointlocationms_x _grabpointlocationms_y) (`KismetMathLibrary.BreakVector` (`local.GrabPointLocationMS`)))
  (bind _closestgrabcomponentonoverlap (`self.ClosestGrabComponentOnOverlap`))
  (bind (_motioncontrollerlocationms_x _motioncontrollerlocationms_y) (`KismetMathLibrary.BreakVector` (`local.MotionControllerLocationMS`)))
  (bind (_grabpointlocationms_x_2 _grabpointlocationms_y_2 _grabpointlocationms_z) (`KismetMathLibrary.BreakVector` (`local.GrabPointLocationMS`)))
  (bind _adjustedclosestgrabpointws (`self.AdjustedClosestGrabPointWS`))
  (bind (_meshcenterlocationms_x _meshcenterlocationms_y) (`KismetMathLibrary.BreakVector` (`local.MeshCenterLocationMS`)))
  (bind (_motioncontrollerlocationms_x_2 _motioncontrollerlocationms_y_2 _motioncontrollerlocationms_z) (`KismetMathLibrary.BreakVector` (`local.MotionControllerLocationMS`)))
  (bind (_grabprofile_proptype _grabprofile_grabdirection) (break `/Game/Core/Grabbable/Structs/S_GrabProfile` (`self.GrabProfile`)))
  (bind _returnvalue (`KismetMathLibrary.Normal` (`KismetMathLibrary.MakeVector` _motioncontrollerlocationms_x _motioncontrollerlocationms_y)))
  (bind _returnvalue_2 (`KismetMathLibrary.Normal` (`KismetMathLibrary.MakeVector` _grabpointlocationms_x _grabpointlocationms_y)))
  (bind _returnvalue_3 (`SceneComponent.K2_GetComponentLocation` (`self.Motion Controller`)))
  (bind (_relativelocation_x _relativelocation_y _relativelocation_z) (`KismetMathLibrary.BreakVector` (`SceneComponent.RelativeLocation` _closestgrabcomponentonoverlap)))
  (bind (_relativerotation_roll _relativerotation_pitch _relativerotation_yaw) (`KismetMathLibrary.BreakRotator` (`SceneComponent.RelativeRotation` (`self.ClosestGrabComponentOnOverlap`))))
  (bind _returnvalue_4 (`KismetMathLibrary.SelectFloat` -1.0 1.0 (`|EnumEquality` (`self.Hand`) "Left")))
  (bind (_returnvalue_x _returnvalue_y _returnvalue_z) (`KismetMathLibrary.BreakVector` (`KismetMathLibrary.Cross_VectorVector` _returnvalue_2 _returnvalue)))
  (bind _returnvalue_5 (`KismetMathLibrary.Vector_Distance` (+ (* (`local.UnitDirectionFromGrabToMC`) (`self.InitialDistanceHandToObj`)) _adjustedclosestgrabpointws) _adjustedclosestgrabpointws))
  (bind _returnvalue_6 (`KismetMathLibrary.MapRangeClamped` (`KismetMathLibrary.Vector_Distance` _returnvalue_3 (`self.AdjustedClosestGrabPointWS`)) 0.0 _returnvalue_5 0.0 1.0))
  (`self.ClosestGrabComponentOnOverlap`
    (:`then`
      (`PrimitiveComponent.SetSimulatePhysics` (`self.Skeletal Mesh`) false)
      (`PrimitiveComponent.SetCollisionEnabled` (`self.Skeletal Mesh`) "QueryOnly")
      (switch `/Game/Core/Grabbable/Enums/E_GrabDirection` _grabprofile_grabdirection
        (:`NewEnumerator1`
          ;[0.05161 0.1165 0.15 0.5] Variables Set
          (set `local.MotionControllerLocationWS` (`SceneComponent.K2_GetComponentLocation` (`self.Motion Controller`)))
          (set `local.GrabPointLocationMS` (`KismetMathLibrary.MakeVector` _relativelocation_x (* _relativelocation_y (`KismetMathLibrary.SelectFloat` -1.0 1.0 (`|EnumEquality` (`self.Hand`) "Left"))) _relativelocation_z))
          (set `local.MeshCenterLocationMS` (0.0 0.0 0.0))
          (set `local.MeshWorldTransform` (`SceneComponent.K2_GetComponentToWorld` (`SceneComponent.GetAttachParent` _closestgrabcomponentonoverlap)))
          (set `local.MotionControllerLocationMS` (`KismetMathLibrary.InverseTransformLocation` (`local.MeshWorldTransform`) (`local.MotionControllerLocationWS`)))
          ;[0.15 0.1284 0.08458 0.5] Angle Between Motion Controller and Grab Poin in MESH SPACE
          (bind _output_get (set `local.AngleBetweenMotionControllerAndGrabPoint` (mod (+ (`KismetMathLibrary.DegAtan2` _returnvalue_z (`KismetMathLibrary.Dot_VectorVector` _returnvalue_2 _returnvalue)) 360.0) 360.0)))
          (bind (_returnvalue_x_2 _returnvalue_y_2) (`KismetMathLibrary.BreakVector` (`KismetMathLibrary.RotateAngleAxis` (`KismetMathLibrary.MakeVector` _grabpointlocationms_x_2 _grabpointlocationms_y_2 _grabpointlocationms_z) _output_get (`KismetMathLibrary.MakeVector` _meshcenterlocationms_x _meshcenterlocationms_y _grabpointlocationms_z))))
          (bind _output_get_2 (set `self.AdjustedGrabPointLocationMS` (`KismetMathLibrary.MakeVector` _returnvalue_x_2 _returnvalue_y_2 _motioncontrollerlocationms_z)))
          (bind _output_get_3 (set `self.AdjustedClosestGrabPointWS` (`KismetMathLibrary.TransformLocation` (`local.MeshWorldTransform`) _output_get_2)))
          (bind _returnvalue_7 (`KismetMathLibrary.GetDirectionUnitVector` _output_get_3 _returnvalue_3))
          (set `local.UnitDirectionFromGrabToMC` _returnvalue_7)
          (set `self.HandDistanceAlpha` (- 1.0 _returnvalue_6))
          (`SceneComponent.K2_SetWorldLocation` (`self.Skeletal Mesh`) (+ _output_get_3 (* (* _returnvalue_7 _returnvalue_6) (* _returnvalue_6 _returnvalue_5))) false false)
          ;[0.111 0.08701 0.15 0.5] Rotate Hand To Obj
          (set `self.AdjustedGrabPointRotation` (`KismetMathLibrary.ComposeRotators` (`KismetMathLibrary.MakeRotator` (* _relativerotation_roll _returnvalue_4) _relativerotation_pitch (* _relativerotation_yaw _returnvalue_4)) (`KismetMathLibrary.MakeRotator` 0.0 0.0 (`local.AngleBetweenMotionControllerAndGrabPoint`))))
          (`SceneComponent.K2_SetWorldRotation` (`self.Skeletal Mesh`) (`KismetMathLibrary.RInterpTo` (`SceneComponent.K2_GetComponentRotation` (`self.Skeletal Mesh`)) (`KismetMathLibrary.TransformRotation` (`local.MeshWorldTransform`) (`self.AdjustedGrabPointRotation`)) (`GameplayStatics.GetWorldDeltaSeconds`) 30.0) false false))))
    (:`else`)))

(fn `SetGrabProfile`
  (bind _closestgrabcomponentonoverlap (`self.ClosestGrabComponentOnOverlap`)
    (:`then`
      (bind _asbpc_grab_component (cast `/Game/Core/Grabbable/BPC_GrabComponent` _closestgrabcomponentonoverlap))
      (set `self.GrabProfile` (`/Game/Core/Grabbable/BPC_GrabComponent.GrabProfile` _asbpc_grab_component)))
    (:`else`)))

(fn `SetHandAnimState`
  (params (HandAnimState :type "/Game/Core/Glove/Animation/Enums/E_HandPoses Enum" :default "NewEnumerator0"))
  (set `self.HandAnimState` HandAnimState))

(fn `SetInitialHandDistance`
  (params (Actor :type "Actor Object Reference"))
  (`/Engine/EditorBlueprintResources/StandardMacros.IsValid` Actor
    (:`Is Valid`
      (bind _asbp_grabbable (cast `/Game/Core/Grabbable/BP_Grabbable` Actor))
      (bind _returnvalue (`Actor.K2_GetActorLocation` _asbp_grabbable))
      (set `self.InitialDistanceHandToObj` (- (`KismetMathLibrary.Vector_Distance` (`SceneComponent.K2_GetComponentLocation` (`self.Motion Controller`)) _returnvalue) (`KismetMathLibrary.Vector_Distance` _returnvalue (`SceneComponent.K2_GetComponentLocation` (`/Game/Core/Grabbable/BP_Grabbable.BPC_Grab_Side` _asbp_grabbable)))))
      (`KismetSystemLibrary.PrintString` "Hello"))))

(fn `SetInitialHandDistanceForTryGrab`
  (set `self.InitialHandToMeshDistance` (`KismetMathLibrary.Vector_Distance` (`SceneComponent.K2_GetComponentLocation` (`self.Skeletal Mesh`)) (`self.AdjustedClosestGrabPointWS`))))

(fn `SetPhysicsControl`
  (`PhysicsControlComponent.CreateNamedControl` (`self.Physics Control`) (`self.PhysicsControlHand`) (`self.Anchor`) "None" (`self.Skeletal Mesh`) "None" (`self.Control Data`) (make `PhysicsControlTarget` (0.0 0.0 0.0)) "None"))

(fn `SetValues`
  (bind _asbp_motion_controller (cast `/Game/Core/Character/BP_MotionController` (`self.GetOwner`)))
  (set `self.Motion Controller` (`/Game/Core/Character/BP_MotionController.MotionControllerGrip` _asbp_motion_controller))
  (set `self.Skeletal Mesh` (`/Game/Core/Character/BP_MotionController.HandMesh` _asbp_motion_controller))
  (set `self.Proximity Sphere` (`/Game/Core/Character/BP_MotionController.ProximitySphere` _asbp_motion_controller))
  (set `self.Hand` (`/Game/Core/Character/BP_MotionController.Hand` _asbp_motion_controller))
  (set `self.Physics Control` (`/Game/Core/Character/BP_MotionController.PhysicsControl` _asbp_motion_controller))
  (set `self.Anchor` (`/Game/Core/Character/BP_MotionController.Anchor` _asbp_motion_controller)))