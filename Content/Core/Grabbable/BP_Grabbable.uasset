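; BP_Grabbable is an actor that finds which of its grab points is closest to a character's hand.
; SetNearestGrabComponent compares the world distance from CharacterHand to each BPC_GrabComponent on the actor and keeps the closest.
; Each replacement saves the prior pick as PrevNearestGrabComponent, and the distance resets to a large sentinel after the loop if a valid pick exists.
; The event graph and construction script are empty.
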(fn `SetNearestGrabComponent`
  (for _array_element (`self.K2_GetComponentsByClass` "/Game/Core/Grabbable/BPC_GrabComponent.BPC_GrabComponent_C")
    (bind _returnvalue (`KismetMathLibrary.VSize` (- (`SceneComponent.K2_GetComponentLocation` (`self.CharacterHand`)) (`SceneComponent.K2_GetComponentLocation` _array_element))))
    (if (< _returnvalue (`self.NearestGrabDistance`))
      (set `self.NearestGrabDistance` _returnvalue)
      (bind _nearestgrabcomponent (`self.NearestGrabComponent`)
        (:`then`
          (set `self.PrevNearestGrabComponent` _nearestgrabcomponent)
          (set `self.NearestGrabComponent` _array_element))
        (:`else`
          (set `self.NearestGrabComponent` _array_element)))))
  (`self.NearestGrabComponent`
    (:`then`
      (set `self.NearestGrabDistance` 100000.0))
    (:`else`)))

(fn `UserConstructionScript`)