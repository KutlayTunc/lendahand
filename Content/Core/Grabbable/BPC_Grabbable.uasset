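; Grabbable actor, apparently for VR, that highlights whichever of its BPC_Grab points is nearest to an overlapping hand.
; ProximityChecker overlap stores the other component as CharacterHand, without a character check, and starts a looping timer at frame-delta interval.
; The timer compares grab-point distances, turning the nearest point's child point light green and the previous one's red.
; End overlap stops the timer and resets the highlight to red.
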(event `self.ProximityChecker.OnComponentBeginOverlap`
  (params (OverlappedComponent :type "PrimitiveComponent Object Reference") (OtherActor :type "Actor Object Reference") (OtherComp :type "PrimitiveComponent Object Reference") (OtherBodyIndex :type Integer) (bFromSweep :type Boolean) (SweepResult :type "HitResult Structure (by ref)"))
  (set `self.CharacterHand` OtherComp)
  (bind _returnvalue (`KismetSystemLibrary.K2_SetTimerDelegate` (delegate `CheckDistance`) (`GameplayStatics.GetWorldDeltaSeconds`) true))
  (set `self.TimerNearestGrabComponent` _returnvalue))

(event `CheckDistance`
  (`self.SetNearestGrabComponent`))

(event `self.ProximityChecker.OnComponentEndOverlap`
  (params (OverlappedComponent :type "PrimitiveComponent Object Reference") (OtherActor :type "Actor Object Reference") (OtherComp :type "PrimitiveComponent Object Reference") (OtherBodyIndex :type Integer))
  (`KismetSystemLibrary.K2_ClearAndInvalidateTimerHandle` (`self.TimerNearestGrabComponent`))
  (set `self.NearestGrabDistance` 100000.0)
  (set `self.PrevNearestGrabComponent` null)
  (bind _nearestgrabcomponent (`self.NearestGrabComponent`)
    (:`then`
      (bind _aspoint_light_component (cast `PointLightComponent` (`SceneComponent.GetChildComponent` _nearestgrabcomponent 0)))
      (`LightComponent.SetLightColor` _aspoint_light_component (struct :`R` 1.0 :`B` 0.103049 :`A` 1.0) true)
      (set `self.NearestGrabComponent` null))
    (:`else`)))

(fn `SetNearestGrabComponent`
  (for _array_element (`self.K2_GetComponentsByClass` "/Game/Core/Grabbable/BPC_Grab.BPC_Grab_C")
    (bind _returnvalue (`KismetMathLibrary.VSize` (- (`SceneComponent.K2_GetComponentLocation` (`self.CharacterHand`)) (`SceneComponent.K2_GetComponentLocation` _array_element))))
    (if (< _returnvalue (`self.NearestGrabDistance`))
      (set `self.NearestGrabDistance` _returnvalue)
      (bind _nearestgrabcomponent (`self.NearestGrabComponent`)
        (:`then`
          (bind _output_get (set `self.PrevNearestGrabComponent` _nearestgrabcomponent))
          (set `self.NearestGrabComponent` _array_element)
          (bind _aspoint_light_component (cast `PointLightComponent` (`SceneComponent.GetChildComponent` _output_get 0)))
          (`LightComponent.SetLightColor` _aspoint_light_component (struct :`R` 1.0 :`B` 0.103049 :`A` 1.0) true))
        (:`else`
          (set `self.NearestGrabComponent` _array_element)))))
  (bind _nearestgrabcomponent_2 (`self.NearestGrabComponent`)
    (:`then`
      (bind _aspoint_light_component_2 (cast `PointLightComponent` (`SceneComponent.GetChildComponent` _nearestgrabcomponent_2 0)))
      (`LightComponent.SetLightColor` _aspoint_light_component_2 (struct :`G` 1.0 :`B` 0.091509 :`A` 1.0) true)
      (set `self.NearestGrabDistance` 100000.0))
    (:`else`)))

(fn `UserConstructionScript`)