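; BP_HandTrackingPawn is a VR pawn for Oculus hand tracking that exposes the bone pose of its right hand component.
; On BeginPlay it sets the tracking origin to Stage.
; GetBoneTransforms clears and rebuilds an array of world-space transforms for every bone of the ROculusXRHand component, looked up by name in index order, and returns it.
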(event `self.ReceiveBeginPlay`
  (`HeadMountedDisplayFunctionLibrary.SetTrackingOrigin` "Stage"))

(fn `GetBoneTransforms`
  (returns (BoneTransforms :type "Array of Transform Structure"))
  (`KismetArrayLibrary.Array_Clear` (`self.BoneTransforms`))
  (for _index (range (`SkinnedMeshComponent.GetNumBones` (`self.R_OculusXRHand`)))
    (bind _returnvalue (`PoseableMeshComponent.GetBoneTransformByName` (`self.R_OculusXRHand`) (`SkinnedMeshComponent.GetBoneName` (`self.R_OculusXRHand`) _index) "WorldSpace"))
    (`KismetArrayLibrary.Array_Add` (`self.BoneTransforms`) _returnvalue))
  (return (`self.BoneTransforms`)))

(fn `UserConstructionScript`)