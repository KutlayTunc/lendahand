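; Hand motion capture Blueprint built around a right-hand OculusXR hand component.
; On BeginPlay it sets the tracking origin to Stage.
; GetBoneTransforms holds logic to collect the world-space transform of each hand bone by name into an array, but that logic is disconnected from the function entry and never runs.
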(event `self.ReceiveBeginPlay`
  (`HeadMountedDisplayFunctionLibrary.SetTrackingOrigin` "Stage"))

(fn `GetBoneTransforms`
  (returns (BoneTransforms :type "Array of Transform Structure")))

(fn `UserConstructionScript`)