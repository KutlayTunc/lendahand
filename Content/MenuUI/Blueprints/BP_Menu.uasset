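; BP_Menu is a world-space menu actor that builds a growing row of BP_MenuPanel actors, adding one at BeginPlay and another on a looping timer.
; Each new panel spawns at the root and attaches to the Anchor, which a timeline slides along negative Y by the panel's width plus a small gap.
; Panels after the first stay hidden until the slide finishes, then all are made visible.
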(event `self.ReceiveBeginPlay`
  (`self.AddNewPanel`)
  (`KismetSystemLibrary.K2_SetTimerDelegate` (delegate `CustomEvent`) 2.0 true))

(event `CustomEvent`
  (`self.AddNewPanel`))

(event `PushPanel`)

(event `PushMenu`
  (params (Vector :type "Vector Structure"))
  (bind _returnvalue (* Vector_Y -2.0))
  (bind _returnvalue_2 (`SceneComponent.K2_GetComponentLocation` (`self.Anchor`)))
  (set `self.InitialLoc` _returnvalue_2)
  (set `self.TargetLoc` (+ _returnvalue_2 (`KismetMathLibrary.MakeVector` 0.0 (+ _returnvalue (/ _returnvalue 10.0)))))
  (bind (_direction _newtrack_0) (`Timeline|Timeline` :!via `PlayFromStart`)
    (:`Update`
      (`SceneComponent.K2_SetWorldLocation` (`self.Anchor`) (`KismetMathLibrary.VLerp` (`self.InitialLoc`) (`self.TargetLoc`) _newtrack_0) false false))
    (:`Finished`
      (for _array_element (`self.PanelArray`)
        (`SceneComponent.SetVisibility` (`/Game/MenuUI/Blueprints/BP_MenuPanel.DefaultSceneRoot` _array_element) true true)))))

(fn `AddNewPanel`
  (bind _returnvalue (`|SpawnActorFromClass` "/Game/MenuUI/Blueprints/BP_MenuPanel.BP_MenuPanel_C" (`SceneComponent.K2_GetComponentToWorld` (`self.DefaultSceneRoot`)) "Undefined" "MultiplyWithRoot" null null))
  (`KismetArrayLibrary.Array_AddUnique` (`self.PanelArray`) _returnvalue)
  (`self.K2_AttachToComponent` _returnvalue (`self.Anchor`) "None" "KeepWorld" "SnapToTarget" "KeepRelative" true)
  (`self.PushMenu` (`.BoxExtent` (`self.GetActorBounds` _returnvalue false false)))
  (if (> (`KismetArrayLibrary.Array_Length` (`self.PanelArray`)) 1)
    (`SceneComponent.SetVisibility` (`/Game/MenuUI/Blueprints/BP_MenuPanel.DefaultSceneRoot` _returnvalue) false true)))

(fn `UserConstructionScript`)